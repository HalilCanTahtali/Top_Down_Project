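; Zombie enemy character that wanders, chases and melees the player, and awards XP when killed.
; Tick-driven logic wanders slowly until the LookArea overlap flags the player, then a line trace gates a faster chase.
; At close range it flags the attack on its animation Blueprint, while hand overlaps deal cooldown-gated damage.
; Taking damage briefly halts movement for a hit reaction, and death removes the capsule before delayed destruction.
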(event `self.ReceiveTick`
  (params (DeltaSeconds :type "Float (single-precision)"))
  (bind _returnvalue (`GameplayStatics.GetPlayerCharacter` 0))
  (bind _zombiehand (`self.zombiehand`))
  (bind _charactermovement (`self.CharacterMovement`))
  (if (`self.amidead?`)
    ;[1 1 1] If he was dead wait 3 sec and disappear
    (`KismetSystemLibrary.Delay` 3.0)
    (`self.K2_DestroyActor`)
    (elif (`self.IsSaw`)
      ;[1 1 1] If saw the player throw line trace
      (bind _outhit (`KismetSystemLibrary.LineTraceSingleForObjects` :`Start` (`self.K2_GetActorLocation`) :`End` (+ (`self.K2_GetActorLocation` (`GameplayStatics.GetPlayerCharacter` 0)) (20.0 20.0 20.0)) :`ObjectTypes` (`|MakeArray` "ObjectTypeQuery3" "ObjectTypeQuery1" :!type "EObjectTypeQuery Enum") :`DrawDebugType` "ForDuration"))
      ;[1 1 1] If lanetrace hit the player then run to player
      (cast `/Game/TopDownBP/Blueprints/TopDownCharacter` (`.HitActor` (`GameplayStatics.BreakHitResult` _outhit)))
      (set `CharacterMovementComponent.MaxWalkSpeed` 400.0 (`self.CharacterMovement`))
      (`AIBlueprintHelperLibrary.SimpleMoveToActor` (`self.GetController`) _returnvalue)
      ;[1 1 1] If close enough
      (if (< (`self.GetDistanceTo` _returnvalue) 200.0)
        ;[1 1 1] Attack the player
        (`/Engine/EditorBlueprintResources/StandardMacros.DoOnce` false :!label _label
          (:`Completed`
            (set `self.InRange` true)
            (bind _aswar_zombie_animation_bp (cast `/Game/Zombie/BluePrint/WarZombieAnimationBP` (`SkeletalMeshComponent.GetAnimInstance` (`self.Mesh`))))
            (set `/Game/Zombie/BluePrint/WarZombieAnimationBP.IsAttacking` true _aswar_zombie_animation_bp)
            (`ActorComponent.SetComponentTickEnabled` _zombiehand true)
            (`KismetSystemLibrary.Delay` 2.63)
            (`ActorComponent.SetComponentTickEnabled` _zombiehand false)
            (set `/Game/Zombie/BluePrint/WarZombieAnimationBP.IsAttacking` false _aswar_zombie_animation_bp)
            (set `self.InRange` false)
            (goto _label :!via `Reset`))))
      (else
        ;[1 1 1] looking for player
        (`KismetSystemLibrary.Delay` (`KismetMathLibrary.RandomFloatInRange` 4.0 5.0))
        (set `CharacterMovementComponent.MaxWalkSpeed` 50.0 _charactermovement)
        (`AIBlueprintHelperLibrary.SimpleMoveToLocation` (`self.GetController`) (`NavigationSystemV1.K2_GetRandomLocationInNavigableRadius` (`self.K2_GetActorLocation`) 500.0 null null))
        (`KismetSystemLibrary.Delay` 2.0)
        (set `CharacterMovementComponent.MaxWalkSpeed` 0.0 _charactermovement)))))

(event `self.LookArea.OnComponentBeginOverlap`
  (params (OverlappedComponent :type "PrimitiveComponent Object Reference") (OtherActor :type "Actor Object Reference") (OtherComp :type "PrimitiveComponent Object Reference") (OtherBodyIndex :type Integer) (bFromSweep :type Boolean) (SweepResult :type "HitResult Structure (by ref)"))
  ;[1 1 1] set the IsSaw veriables if the player inside at lookarea collision
  (cast `/Game/TopDownBP/Blueprints/TopDownCharacter` OtherActor)
  (set `self.IsSaw` true))

(event `self.LookArea.OnComponentEndOverlap`
  (params (OverlappedComponent :type "PrimitiveComponent Object Reference") (OtherActor :type "Actor Object Reference") (OtherComp :type "PrimitiveComponent Object Reference") (OtherBodyIndex :type Integer))
  ;[1 1 1] set the IsSaw veriables if the player inside at lookarea collision
  (cast `/Game/TopDownBP/Blueprints/TopDownCharacter` OtherActor)
  (set `self.IsSaw` false))

(event `self.zombiehand.OnComponentBeginOverlap`
  (params (OverlappedComponent :type "PrimitiveComponent Object Reference") (OtherActor :type "Actor Object Reference") (OtherComp :type "PrimitiveComponent Object Reference") (OtherBodyIndex :type Integer) (bFromSweep :type Boolean) (SweepResult :type "HitResult Structure (by ref)"))
  ;[1 1 1] If zombie hand hit the player capsule component give damage the player but not always just every zombie attack anim playing
  (bind _astop_down_character (cast `/Game/TopDownBP/Blueprints/TopDownCharacter` OtherActor))
  (`/Engine/EditorBlueprintResources/StandardMacros.DoOnce` false :!label _label_2
    (:`Completed`
      (`GameplayStatics.ApplyDamage` _astop_down_character 20.0 null self "/Script/Engine.DamageType")
      (`KismetSystemLibrary.Delay` 3.0)
      (goto _label_2 :!via `Reset`))))

(event `self.ReceiveAnyDamage`
  (params (Damage :type "Float (single-precision)") (DamageType :type "DamageType Object Reference") (InstigatedBy :type "Controller Object Reference") (DamageCauser :type "Actor Object Reference"))
  (bind _charactermovement (`self.CharacterMovement`))
  ;[1 1 1] Take damage
  (set `self.Health` (- (`self.Health`) Damage))
  ;;[0.1876 1 0.447] Play death anim if health <=0
  (if (<= (`self.Health`) 0.0)
    (set `self.amidead?` true)
    (`ActorComponent.K2_DestroyComponent` (`self.CapsuleComponent`))
    ;;[1 0.9544 0] add xp to player
    (bind _astop_down_character (cast `/Game/TopDownBP/Blueprints/TopDownCharacter` (`GameplayStatics.GetPlayerCharacter` 0)))
    (`/Game/TopDownBP/Blueprints/TopDownCharacter.AddXP` _astop_down_character 40.0))
  ;;[0.2541 0.3275 1] if take damage delay 1.17 sec for playing take damage anim
  (set `self.takedamage?` true)
  (`CharacterMovementComponent.SetMovementMode` _charactermovement "MOVE_None" 0)
  (`KismetSystemLibrary.Delay` 1.17)
  (`CharacterMovementComponent.SetMovementMode` _charactermovement "MOVE_Walking" 0)
  (set `self.takedamage?` false))

(fn `UserConstructionScript`)